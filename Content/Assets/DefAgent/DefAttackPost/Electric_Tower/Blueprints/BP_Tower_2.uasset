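; BP_Tower_2 is an electric defence tower that reacts to BP_TargetActor instances entering and leaving its sphere trigger.
; On entry it flags the target as in range, then spawns a BP_ElectricArc at the Start component, aims it at that target and starts it.
; On exit it clears the flag and calls DamageRegeneration on the target.
; An overlap counter scales the mesh's "Multiply" material parameter, so the tower glows brighter with each target inside.
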(event OnComponentBeginOverlap(Sphere)
  (params (OverlappedComponent :type Primitive%20Component%20Object%20Reference) (OtherActor :type Actor%20Object%20Reference) (OtherComp :type Primitive%20Component%20Object%20Reference) (OtherBodyIndex :type Integer) (bFromSweep :type Boolean) (SweepResult :type Hit%20Result%20Structure%20%28by%20ref%29))
  ;[1 1 1] When the target actor is in range
  (bind _asbp_target_actor (Utilities|Casting|CastToBP_TargetActor OtherActor))
  (Variables|/Game/Electric_Tower/Blueprints/BP_TargetActor.BP_TargetActor_C|SetInRange _asbp_target_actor true)
  ;[1 1 1] Spanw Electric Arcs
  (bind _returnvalue (Game|SpawnActorfromClass "/Game/Electric_Tower/Blueprints/BP_ElectricArc.BP_ElectricArc_C" (Math|Transform|MakeTransform (Transformation|GetWorldLocation (Variables|Default|GetStart)) "0, 0, 0" "1,1,1") "Undefined" 0 0))
  (Variables|/Game/Electric_Tower/Blueprints/BP_ElectricArc.BP_ElectricArc_C|SetTargetActor _returnvalue _asbp_target_actor)
  (Default|Start _returnvalue)
  ;[1 1 1] Increase tower light
  (bind _result (Math|Float|IncrementFloat (Variables|Default|GetMatEmissive))
    (:%20%20
      (bind _output_get (Variables|Default|SetMatEmissive _result))
      (Rendering|Material|SetScalarParameterValueonMaterials (Variables|Default|GetSM_Tower_1) "Multiply" (* _output_get 5.0)))))

(event OnComponentEndOverlap(Sphere)
  (params (OverlappedComponent :type Primitive%20Component%20Object%20Reference) (OtherActor :type Actor%20Object%20Reference) (OtherComp :type Primitive%20Component%20Object%20Reference) (OtherBodyIndex :type Integer))
  ;[1 1 1] When Target Actor is out of range, recharge health
  (bind _asbp_target_actor (Utilities|Casting|CastToBP_TargetActor OtherActor))
  (Variables|/Game/Electric_Tower/Blueprints/BP_TargetActor.BP_TargetActor_C|SetInRange _asbp_target_actor false)
  (Default|DamageRegeneration _asbp_target_actor)
  ;[1 1 1] Reduce tower light
  (bind _result (Math|Float|DecrementFloat (Variables|Default|GetMatEmissive))
    (:%20%20
      (bind _output_get (Variables|Default|SetMatEmissive _result))
      (Rendering|Material|SetScalarParameterValueonMaterials (Variables|Default|GetSM_Tower_1) "Multiply" (* _output_get 5.0)))))

(fn ConstructionScript)