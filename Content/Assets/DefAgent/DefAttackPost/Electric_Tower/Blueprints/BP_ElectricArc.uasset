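; BP_ElectricArc is the Electric Tower's beam actor, arcing to a target and damaging it while in range.
; Construction collapses the Niagara beam's end point onto its own origin.
; Start runs a short Delay loop that moves the beam end to TargetActor and calls its Damage each pass.
; An invalid target gets one delayed recheck; failing that, or leaving range, stops the electric cue and destroys the arc.
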(event Custom|Start
  (bind _targetactor (Variables|Default|GetTargetActor))
  ;[1 1 1] Start Electric Beam
  ;[1 1 1] Target Actor control
  (Utilities|IsValid _targetactor :!label _label
    (:Is%20Valid
      ;[1 1 1] Range check
      (if (Variables|/Game/Electric_Tower/Blueprints/BP_TargetActor.BP_TargetActor_C|GetInRange _targetactor) :!label _label_2
        ;[1 1 1] Set Beam Endpoint
        (Effects|Components|ParticleSystem|SetVectorParameter (Variables|Default|GetNiagara) "User.BeamEnd" (Transformation|GetActorLocation _targetactor))
        (Default|Damage _targetactor)
        (Utilities|FlowControl|Delay 0.01)
        (goto _label)
        (else
          _)))
    (:Is%20Not%20Valid
      ;[1 1 1] Target Actor control again
      (Utilities|FlowControl|Delay 0.3)
      (Utilities|IsValid _targetactor
        (:Is%20Valid
          (goto _label_2))
        (:Is%20Not%20Valid
          _))))
  (Audio|Components|Audio|Stop (Variables|Default|GetCue_Electric))
  (Actor|DestroyActor))

(fn ConstructionScript
  (bind _niagara (Variables|Default|GetNiagara))
  (Effects|Components|ParticleSystem|SetVectorParameter _niagara "User.BeamEnd" (Transformation|GetWorldLocation _niagara)))