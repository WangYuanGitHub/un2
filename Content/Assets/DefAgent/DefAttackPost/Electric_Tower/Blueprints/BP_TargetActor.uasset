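; BP_TargetActor is a destructible target in the Electric Tower assets that glows brighter as it takes damage.
; Each Damage call raises the sphere material's "Multiply" emissive parameter and lowers Health, then spawns explosion effects and destroys the actor once Health runs out.
; DamageRegeneration uses a short Delay loop to fade the glow while InRange is false, without restoring Health.
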(event Custom|Damage
  (bind _returnvalue (Transformation|GetActorLocation))
  ;[1 1 1] Increase the actor emissive
  (if (< (Variables|Default|GetMatEmissive) 1e+02)
    (bind _result (Math|Float|IncrementFloat (Variables|Default|GetMatEmissive))
      (:%20%20
        (Variables|Default|SetMatEmissive _result)))
    (else
      (Variables|Default|SetMatEmissive 1e+02)))
  (Rendering|Material|SetScalarParameterValueonMaterials (Variables|Default|GetSphere) "Multiply" _result)
  ;[1 1 1] Reduce Heath
  (bind _result_2 (Math|Float|DecrementFloat (Variables|Default|GetHealth))
    (:%20%20
      (bind _output_get (Variables|Default|SetHealth _result_2))
      ;[1 1 1] Kill Actor if healt is bellow 0
      (if (<= _output_get 0.0)
        (Effects|SpawnEmitteratLocation "/Game/Electric_Tower/Particles/P_Explosion.P_Explosion" _returnvalue "0, 0, 0" "3.000000,3.000000,3.000000")
        (Audio|SpawnSoundatLocation "/Game/Electric_Tower/Sounds/S_Explosion.S_Explosion" _returnvalue "0, 0, 0" 1.0 1.0 0.0 0 0)
        (Actor|DestroyActor)))))

(event Custom|DamageRegeneration
  ;[1 1 1] To revert to the old view by reducing the Emissive value
  (if (not (Variables|Default|GetInRange)) :!label _label
    (if (not (<= (Variables|Default|GetMatEmissive) 0.0))
      (bind _output_get (Variables|Default|SetMatEmissive (- (Variables|Default|GetMatEmissive) 5.0)))
      (Rendering|Material|SetScalarParameterValueonMaterials (Variables|Default|GetSphere) "Multiply" _output_get)
      (Utilities|FlowControl|Delay 0.01)
      (goto _label))))

(fn ConstructionScript)